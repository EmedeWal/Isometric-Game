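; Player controller for click-to-move navigation that registers the default Enhanced Input mapping context on BeginPlay.
; While the destination input is triggered, it projects the cursor's trace hit onto the navmesh and moves there with SimpleMoveToLocation.
; A short click also spawns cursor VFX at the destination, choosing the invalid effect when a synchronous path query returns a partial path.
; A separate stop action halts movement.
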(event `self.ReceiveBeginPlay`
  (bind _returnvalue (subsystem `EnhancedInputLocalPlayerSubsystem`))
  ;[0.05098 0.05098 0.05098] Add Mapping Context
  (`/Engine/EditorBlueprintResources/StandardMacros.IsValid` _returnvalue
    (:`Is Valid`
      (`EnhancedInputSubsystemInterface.AddMappingContext` _returnvalue "/Game/Player/Input/IMC_Default.IMC_Default" 0 (struct)))
    (:`Is Not Valid`
      (`KismetSystemLibrary.PrintString` "IMC is not valid!"))))

(event `EnhancedInput|/Game/Player/Input/Actions/IA_SetDestination`
  (params (ActionValue :type Boolean) (ElapsedSeconds :type "Float (double-precision)") (TriggeredSeconds :type "Float (double-precision)") (InputAction :type "InputAction Object Reference" :default "/Game/Player/Input/Actions/IA_SetDestination.IA_SetDestination"))
  ;[0.05098 0.05098 0.05098] Handle Movement
  (:`Triggered`
    (bind (_destination _successful) (`self.Set Controller Destination`)))
  (:`Completed`
    (if (and _successful (< TriggeredSeconds (`self.MinClickHoldTime`)))
      (`self.Destination Set` _destination))))

(event `EnhancedInput|/Game/Player/Input/Actions/IA_StopActions`
  (params (ActionValue :type Boolean) (ElapsedSeconds :type "Float (double-precision)") (TriggeredSeconds :type "Float (double-precision)") (InputAction :type "InputAction Object Reference" :default "/Game/Player/Input/Actions/IA_StopActions.IA_StopActions"))
  ;[0.05098 0.05098 0.05098] Stop Action Handling
  (:`Triggered`
    (`self.StopMovement`)))

(event `Destination Updated`
  (params (Destination :type "Vector Structure"))
  ;[0.05098 0.05098 0.05098] Feedback Handling
)

(event `Destination Set`
  (params (Destination :type "Vector Structure"))
  ;[0.05098 0.05098 0.05098] Feedback Handling
  (`self.Spawn Cursor VFX` Destination))

(fn `Get Cursor Location`
  (returns (Location :type "Vector Structure"))
  (bind (_bblockinghit _binitialoverlap _time _distance _location) (`GameplayStatics.BreakHitResult` (`self.GetHitResultUnderCursorByChannel` "TraceTypeQuery1")))
  (if _bblockinghit
    (return _location)))

(fn `Set Controller Destination`
  (returns (Destination :type "Vector Structure") (Successful :type Boolean))
  (locals (`Found Position` :type Boolean))
  (bind _location (`self.Get Cursor Location`))
  (bind (_projectedlocation _returnvalue) (`NavigationSystemV1.K2_ProjectPointToNavigation` _location null null (`self.SampleSize`)))
  (bind _output_get (set `local.Found Position` _returnvalue))
  (if _output_get
    (`AIBlueprintHelperLibrary.SimpleMoveToLocation` self _projectedlocation)
    (`self.Destination Updated` _projectedlocation)
    (else
      (`KismetSystemLibrary.PrintString` "Failed to sample position!" true true (struct :`R` 1.0 :`G` 0.022139 :`B` 8.7e-05 :`A` 1.0))))
  (return _projectedlocation (`local.Found Position`)))

(fn `Spawn Cursor VFX`
  (params (Destination :type "Vector Structure"))
  (locals (SelectedVFX :type "NiagaraSystem Object Reference"))
  (bind _returnvalue (`GameplayStatics.GetPlayerPawn` 0))
  (bind _returnvalue_2 (`NavigationSystemV1.FindPathToLocationSynchronously` (`Pawn.GetNavAgentLocation` _returnvalue) Destination _returnvalue null))
  (if (`NavigationPath.IsPartial` _returnvalue_2)
    (set `local.SelectedVFX` (`self.InvalidClickVFX`))
    (else
      (set `local.SelectedVFX` (`self.ValidClickVFX`))))
  (`NiagaraFunctionLibrary.SpawnSystemAtLocation` (`local.SelectedVFX`) Destination))

(fn `UserConstructionScript`)