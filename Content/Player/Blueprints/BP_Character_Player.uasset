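; Player character Blueprint that provides smoothed scroll-wheel zoom for its spring-arm camera.
; On BeginPlay the arm starts midway between its minimum and maximum lengths.
; The Enhanced Input scroll action offsets the current arm length by zoom speed and clamps it into a target.
; Tick lerps the spring arm toward that target using delta time scaled by a smoothing factor.
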(event `self.ReceiveBeginPlay`
  (`self.SetInitialArmLength`))

(event `self.ReceiveTick`
  (params (DeltaSeconds :type "Float (single-precision)"))
  (`self.LerpTargetArmLength` DeltaSeconds))

(event `EnhancedInput|/Game/Player/Input/Actions/IA_ScrollZoom`
  (params (ActionValue :type "Float (double-precision)") (ElapsedSeconds :type "Float (double-precision)") (TriggeredSeconds :type "Float (double-precision)") (InputAction :type "InputAction Object Reference" :default "/Game/Player/Input/Actions/IA_ScrollZoom.IA_ScrollZoom"))
  (:`Triggered`
    (`self.SetTargetArmLength` ActionValue)))

(fn `LerpTargetArmLength`
  (params (DeltaTime :type "Float (double-precision)"))
  (bind _springarm (`self.SpringArm`))
  (set `SpringArmComponent.TargetArmLength` (`KismetMathLibrary.Lerp` (`SpringArmComponent.TargetArmLength` _springarm) (`self.TargetArmLength`) (* DeltaTime (`self.ZoomSmoothing`))) _springarm))

(fn `SetInitialArmLength`
  (bind _output_get (set `self.TargetArmLength` (/ (+ (`self.MinSpringArmLength`) (`self.MaxSpringArmLength`)) 2.0)))
  (set `SpringArmComponent.TargetArmLength` _output_get (`self.SpringArm`)))

(fn `SetTargetArmLength`
  (params (Value :type "Float (double-precision)"))
  (set `self.TargetArmLength` (`KismetMathLibrary.FClamp` (- (`SpringArmComponent.TargetArmLength` (`self.SpringArm`)) (* Value (`self.ZoomSpeed`))) (`self.MinSpringArmLength`) (`self.MaxSpringArmLength`))))

(fn `UserConstructionScript`)